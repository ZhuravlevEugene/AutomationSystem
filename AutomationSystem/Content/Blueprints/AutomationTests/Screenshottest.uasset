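; Screenshot test Blueprint for automation testing that captures a gameplay screenshot and then finishes.
; On test start it takes a screenshot with default gameplay options at low tolerance and a short delay, then reports success.
; Unconnected leftover nodes hold alternative captures, including one from a camera actor, and a GroundTruth modifiability print, none of which run.
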(event EventStartTest
  (Class|AutomationBlueprintFunctionLibrary|TakeAutomationScreenshot "Automated screenshot" "" (Class|AutomationBlueprintFunctionLibrary|GetDefaultScreenshotOptionsforGameplay "Low" 0.2))
  (Class|FunctionalTest|FinishTest "Succeeded" "Test over!"))

(fn ConstructionScript)